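; BP_RenderTarget saves render target captures as timestamped image files on PC and passes the file name on to PlayFab.
; F_SaveCapture_Event builds a "capture.png" name from the current date and time, then exports RT_Target to the project's Content/Capture folder.
; It then casts the Game Instance to PlayFab_InstanceDatabaseConnect and sends only that file name, with MemoryWidget as target, to update capture image data.
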(event Custom|F_SaveCapture_Event
  (bind _returnvalue (Math|DateTime|Now))
  (bind (_year _month _day _hour _minute _second) (Math|DateTime|BreakDateTime _returnvalue))
  ;[0.5165 0.2325 1 0.422] Render and Export On PC
  (Variables|Default|SetFileName (Utilities|String|Append (Utilities|String|ToString(Integer) _year) (Utilities|String|ToString(Integer) _month) (Utilities|String|ToString(Integer) _day) (Utilities|String|ToString(Integer) _hour) (Utilities|String|ToString(Integer) _minute) (Utilities|String|ToString(Integer) _second) "capture.png"))
  (Rendering|ExportRenderTarget "/Game/MemoryAssets/RT_Target.RT_Target" (Utilities|String|Append (Class|KismetSystemLibrary|GetProjectDirectory) "/Content/Capture") (Variables|Default|GetFileName))
  (bind _asplay_fab_instance_database_connect (Utilities|Casting|CastToPlayFab_InstanceDatabaseConnect (Game|GetGameInstance)))
  (Default|PlayFabUpdateCaptureImageDataEvent _asplay_fab_instance_database_connect (Variables|Default|GetFileName) (Variables|Default|GetMemoryWidget)))

(fn ConstructionScript)