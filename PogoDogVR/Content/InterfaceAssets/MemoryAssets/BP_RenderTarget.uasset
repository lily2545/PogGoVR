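; Render target Blueprint that saves a memory snapshot and credits the player's profile for it.
; On the save event, it captures the scene and exports RT_Target to the project's Content/Capture folder under a timestamped name.
; The PlayFab game instance stores the filename, then reloads the profile, with a delay loop polling until finished.
; If this activity was not already done, it increments activity and relationship counters, updates PlayFab and plays CheckMark.
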(event Custom|F_SaveCapture_Event
  (bind _returnvalue (Math|DateTime|Now))
  (bind (_year _month _day _hour _minute _second) (Math|DateTime|BreakDateTime _returnvalue))
  ;[0.5165 0.2325 1 0.422] Render and Export On PC
  (Rendering|SceneCapture|CaptureScene (Variables|Default|GetSceneCaptureComponent2D) :!class /Script/Engine.SceneCaptureComponent2D)
  (Variables|Default|SetFileName (Utilities|String|Append (Utilities|String|ToString(Integer) _year) (Utilities|String|ToString(Integer) _month) (Utilities|String|ToString(Integer) _day) (Utilities|String|ToString(Integer) _hour) (Utilities|String|ToString(Integer) _minute) (Utilities|String|ToString(Integer) _second) "capture.png"))
  (Rendering|ExportRenderTarget "/Game/InterfaceAssets/MemoryAssets/RT_Target.RT_Target" (Utilities|String|Append (Class|KismetSystemLibrary|GetProjectDirectory) "\\Content\\Capture") (Variables|Default|GetFileName))
  (bind _asplay_fab_instance_database_connect (Utilities|Casting|CastToPlayFab_InstanceDatabaseConnect (Game|GetGameInstance)))
  (Default|PlayFabUpdateCaptureImageDataEvent _asplay_fab_instance_database_connect (Variables|Default|GetFileName) (Variables|Default|GetMemoryWidget))
  ;[1 0.1152 0 0.714] Update Profile
  (Variables|/Game/LoginAssets/PlayFab_InstanceDatabaseConnect.PlayFab_InstanceDatabaseConnect_C|SetFinishRun _asplay_fab_instance_database_connect false)
  (Default|PlayFabAcessProfileDataEvent _asplay_fab_instance_database_connect)
  (if (Variables|/Game/LoginAssets/PlayFab_InstanceDatabaseConnect.PlayFab_InstanceDatabaseConnect_C|GetFinishRun _asplay_fab_instance_database_connect) :!label _label
    (if (not (Utilities|Array|Get(acopy) (Variables|/Game/LoginAssets/PlayFab_InstanceDatabaseConnect.PlayFab_InstanceDatabaseConnect_C|GetActivityDoneList _asplay_fab_instance_database_connect) 6))
      (Math|Integer|IncrementInt (Variables|/Game/LoginAssets/PlayFab_InstanceDatabaseConnect.PlayFab_InstanceDatabaseConnect_C|GetActivityDone _asplay_fab_instance_database_connect)
        (:%20%20
          (Math|Integer|IncrementInt (Variables|/Game/LoginAssets/PlayFab_InstanceDatabaseConnect.PlayFab_InstanceDatabaseConnect_C|GetRelashionshipPoint _asplay_fab_instance_database_connect)
            (:%20%20
              (Utilities|Array|SetArrayElem (Variables|/Game/LoginAssets/PlayFab_InstanceDatabaseConnect.PlayFab_InstanceDatabaseConnect_C|GetActivityDoneList _asplay_fab_instance_database_connect) 6 true)
              (Variables|/Game/LoginAssets/PlayFab_InstanceDatabaseConnect.PlayFab_InstanceDatabaseConnect_C|SetFinishRun _asplay_fab_instance_database_connect false)
              (Default|PlayFabUpdateProfileDataEvent _asplay_fab_instance_database_connect)
              (Audio|Components|Audio|Play (Variables|Default|GetCheckMark) 0.0))))))
    (else
      (Utilities|FlowControl|Delay 0.2)
      (goto _label))))

(fn ConstructionScript)